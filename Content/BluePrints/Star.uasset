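; Star actor that randomizes its own size and placement, with all logic in the Construction Script and an empty event graph.
; The script gives the static mesh a random uniform world scale and a dynamic StarFresnel material instance, stored in InstanceMaterial.
; It then pushes the Sphere component a fixed distance in a random direction, so stars can scatter over a spherical shell around their origins.
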(event EventBeginPlay)

(event Collision|EventActorBeginOverlap
  (params (OtherActor :type Actor%20Object%20Reference)))

(event EventTick
  (params (DeltaSeconds :type Float%20%28single-precision%29)))

(fn ConstructionScript
  (Utilities|FlowControl|Sequence
    (:then_0
      (Transformation|SetWorldScale3D (Variables|Default|GetStaticMesh) (Math|Conversions|ToVector(Float) (* (Math|Random|RandomFloat) 1e+02))))
    (:then_1
      (bind _returnvalue (Rendering|Material|CreateDynamicMaterialInstance (Variables|Default|GetStaticMesh) 0 "/Game/Materials/StarFresnel.StarFresnel" "None" :!class /Script/Engine.PrimitiveComponent))
      (Variables|Default|SetInstanceMaterial _returnvalue))
    (:then_2
      (Transformation|AddLocalOffset (Variables|Default|GetSphere) (* (Math|Random|RandomUnitVector) 6e+03) false false))))